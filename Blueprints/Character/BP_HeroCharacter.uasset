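; Player hero character for an RPG, handling pickup name display, weapon equipping and attack input.
; Light attack activates the selected ability through an ability system component initialised after a short delay, while heavy attack only prints a placeholder.
; Overlapped pickups show names via the player controller; GetItemInfo equips a weapon if none is held, and its RepNotify attaches it to the hand socket.
; It also exposes walk speed and melee montage info.
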(event `CL_Handle Pickup Name`
  (params (Pickup :type "Actor Object Reference") (bIsOverlapping :type Boolean))
  (`self.F_Handle Pickup Name` Pickup bIsOverlapping))

(event `InputAction|Light Attack`
  (params (Key :type "Key Structure"))
  (:`Pressed`
    (`/Game/Blueprints/Character/BP_AbilitySystemActorComponent.Try To Activate Ability` (`self.BP_AbilitySystemActorComponent`) (`self.Selected Ability`))))

(event `InputAction|Heavy Attack`
  (params (Key :type "Key Structure"))
  (:`Pressed`
    (`KismetSystemLibrary.PrintString` "Heavy Attack")))

(event `self.ReceiveBeginPlay`
  (`KismetSystemLibrary.Delay` 1.0)
  (`/Game/Blueprints/Character/BP_AbilitySystemActorComponent.Init` (`self.BP_AbilitySystemActorComponent`)))

(event `Get Item Info`
  (`/Engine/EditorBlueprintResources/StandardMacros.IsValid` (`self.Current Displayed Item`)
    (:`Is Valid`
      (`KismetSystemLibrary.PrintString` "Overlapping an item")
      (bind _pickupref (message `/Game/Blueprints/Interfaces/INT_BasePickup.Base Pickup Ref` (`self.Current Displayed Item`)))
      (if (`PickupBase.bIsWeapon` _pickupref)
        (`/Engine/EditorBlueprintResources/StandardMacros.IsValid` (`self.Equipped Weapon`)
          (:`Is Not Valid`
            (`self.Equip Weapon` (`self.Current Displayed Item`))))))
    (:`Is Not Valid`
      (`KismetSystemLibrary.PrintString` "NOT Overlapping an item"))))

(event `/Game/Blueprints/Interfaces/INT_HeroCharacter.SetPlayerSpeed`
  (params (Speed :type "Float (single-precision)"))
  (set `CharacterMovementComponent.MaxWalkSpeed` Speed (`self.CharacterMovement`)))

(event `Equip Weapon`
  (params (Weapon :type "Actor Object Reference"))
  (set `self.Equipped Weapon` Weapon)
  (message `/Game/Blueprints/Interfaces/INT_BasePickup.Disable Physics` (`self.Current Displayed Item`)))

(fn `F_Handle Pickup Name`
  (params (Pickup :type "Actor Object Reference") (bIsOverlapping :type Boolean))
  (if bIsOverlapping
    (bind _output_get (set `self.Current Displayed Item` Pickup))
    (bind _item_name (message `/Game/Blueprints/Interfaces/INT_BasePickup.Item Name` _output_get))
    (bind _pcref (message `/Game/Blueprints/Interfaces/INT_RPGController.PCRPGRef` (`self.GetController`)))
    (`/Game/Blueprints/BP_RPGPlayerController.F_ShowPickupName` _pcref _item_name)
    (else
      (set `self.Current Displayed Item` null)
      (bind _pcref_2 (message `/Game/Blueprints/Interfaces/INT_RPGController.PCRPGRef` (`self.GetController`)))
      (`/Game/Blueprints/BP_RPGPlayerController.F_Hide Pickup name` _pcref_2))))

(fn `Get Melee Attack Info`
  (returns (Montage :type "AnimMontage Object Reference") (Length :type "Float (double-precision)"))
  (locals (L_Montage :type "AnimMontage Object Reference"))
  (bind _output_get (set `local.L_Montage` "/Game/Blueprints/Animations/Basic_Melee_Montage.Basic_Melee_Montage"))
  (bind _returnvalue (`AnimSequenceBase.GetPlayLength` _output_get))
  (return _output_get _returnvalue))

(fn `HeroCharacterRef`
  (returns (CharacterRef :type "/Blueprints/Character/BP_HeroCharacter Object Reference"))
  (return self))

(fn `OnRep_Equipped Weapon`
  (`self.K2_AttachToComponent` (`self.Equipped Weapon`) (`self.Mesh`) "Weapon_R" "SnapToTarget" "SnapToTarget" "SnapToTarget" false))

(fn `UserConstructionScript`)