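; Actor component that handles ability activation for the hero character, currently implementing only a basic melee attack.
; Init caches the owning hero through an interface-style message call.
; TryToActivateAbility switches on the requested ability, blocking melee while unarmed or already attacking, then plays the montage supplied by the hero's melee attack info.
; The attacking flag clears only on montage completion, with no handling for interruption, and debug prints trace each step.
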(event `Try To Activate Ability`
  (params (`Selected Ability` :type "ESelectedAbility Enum" :default "None"))
  (bind _playerref (`self.PlayerRef`))
  (bind _playerref_2 (`self.PlayerRef`))
  (`/Engine/EditorBlueprintResources/StandardMacros.IsValid` _playerref_2
    (:`Is Valid`
      (switch `ESelectedAbility` `Selected Ability`
        (:`Basic_Melee`
          (if (and (not (`self.bIsAttacking`)) (not (`BaseCharacter.bIsUnarmed` _playerref_2)))
            (`KismetSystemLibrary.PrintString` "Melee Attack")
            (set `self.bIsAttacking` true)
            (bind _montage (message `/Game/Blueprints/Interfaces/INT_HeroCharacter.Get Melee Attack Info` _playerref))
            (`|PlayMontage` (`Character.Mesh` _playerref) _montage
              (:`OnCompleted`
                (set `self.bIsAttacking` false)
                (`KismetSystemLibrary.PrintString` "Melee Attack Done")))
            (else
              (`KismetSystemLibrary.PrintString` "Melee Attack in Progress or You're unarmed"))))))))

(event `Init`
  (`KismetSystemLibrary.PrintString` "Abilities are online" true true (struct :`R` 1.0 :`G` 0.060593 :`B` 0.030746 :`A` 1.0))
  (bind _characterref (message `/Game/Blueprints/Interfaces/INT_HeroCharacter.HeroCharacterRef` (`self.GetOwner`)))
  (set `self.PlayerRef` _characterref))