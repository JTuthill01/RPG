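; Base Blueprint for pickups that notifies hero characters when they enter or leave its range.
; Collision sphere overlaps run only on authority, identify the hero through an interface message, and call its pickup-name handler with the overlap state.
; Interface-style getters expose the pickup reference and item name, avoiding casts.
; A separate event turns off the mesh's physics simulation and collision.
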(event `/Game/Blueprints/Interfaces/INT_BasePickup.Disable Physics`
  (`PrimitiveComponent.SetSimulatePhysics` (`self.PickupMesh`) false)
  (`PrimitiveComponent.SetCollisionEnabled` (`self.PickupMesh`) "NoCollision"))

(event `self.Collision Sphere.OnComponentBeginOverlap`
  (params (OverlappedComponent :type "PrimitiveComponent Object Reference") (OtherActor :type "Actor Object Reference") (OtherComp :type "PrimitiveComponent Object Reference") (OtherBodyIndex :type Integer) (bFromSweep :type Boolean) (SweepResult :type "HitResult Structure (by ref)"))
  (`/Engine/EditorBlueprintResources/ActorMacros.Switch Has Authority`
    (:`Authority`
      (bind _characterref (message `/Game/Blueprints/Interfaces/INT_HeroCharacter.HeroCharacterRef` OtherActor))
      (if (== _characterref OtherActor)
        (`/Game/Blueprints/Character/BP_HeroCharacter.CL_Handle Pickup Name` _characterref self true)))))

(event `self.Collision Sphere.OnComponentEndOverlap`
  (params (OverlappedComponent :type "PrimitiveComponent Object Reference") (OtherActor :type "Actor Object Reference") (OtherComp :type "PrimitiveComponent Object Reference") (OtherBodyIndex :type Integer))
  (`/Engine/EditorBlueprintResources/ActorMacros.Switch Has Authority`
    (:`Authority`
      (bind _characterref (message `/Game/Blueprints/Interfaces/INT_HeroCharacter.HeroCharacterRef` OtherActor))
      (if (== _characterref OtherActor)
        (`/Game/Blueprints/Character/BP_HeroCharacter.CL_Handle Pickup Name` _characterref self false)))))

(fn `Base Pickup Ref`
  (returns (PickupRef :type "/Blueprints/Pickup/BP_BasePickup Object Reference"))
  (return self))

(fn `Item Name`
  (returns (`Item Name` :type Text))
  (return (`self.PickupName`)))

(fn `UserConstructionScript`)